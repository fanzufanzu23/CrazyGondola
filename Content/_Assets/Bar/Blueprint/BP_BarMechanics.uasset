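; Bar event station for the gondola game that runs a countdown while active.
; Activate starts the timer and reveals a spotlight, trigger sphere and timer widget, which Tick keeps updated.
; On expiry, Deactivate hides these, resets the timer and returns the bar to the CrazyGondolaGame event list.
; The trigger sphere tells BP_ThirdPersonCharacter when it enters or exits the event zone.
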(event OnComponentBeginOverlap(TriggerSphere)
  (params (OverlappedComponent :type Primitive%20Component%20Object%20Reference) (OtherActor :type Actor%20Object%20Reference) (OtherComp :type Primitive%20Component%20Object%20Reference) (OtherBodyIndex :type Integer) (bFromSweep :type Boolean) (SweepResult :type Hit%20Result%20Structure%20%28by%20ref%29))
  (bind _asbp_third_person_character (Utilities|Casting|CastToBP_ThirdPersonCharacter OtherActor))
  (Default|EnterEventZone _asbp_third_person_character self))

(event OnComponentEndOverlap(TriggerSphere)
  (params (OverlappedComponent :type Primitive%20Component%20Object%20Reference) (OtherActor :type Actor%20Object%20Reference) (OtherComp :type Primitive%20Component%20Object%20Reference) (OtherBodyIndex :type Integer))
  (bind _asbp_third_person_character (Utilities|Casting|CastToBP_ThirdPersonCharacter OtherActor))
  (Default|ExitEventZone _asbp_third_person_character))

(event Custom|Activate
  (Variables|Default|SetTimer (Variables|Default|GetTimerDefault))
  (Variables|Default|SetIsActive true)
  (CallFunction|ActivateSpotlight)
  (Development|SetHiddeninGame (Variables|Default|GetBarTimer) false false))

(event Custom|Deactivate
  (Variables|Default|SetIsActive false)
  (Variables|Default|SetTimer (Variables|Default|GetTimerDefault))
  (bind _ascrazy_gondola_game (Utilities|Casting|CastToCrazyGondolaGame (Game|GetGameMode)))
  (Default|AddEventtoList _ascrazy_gondola_game self)
  (CallFunction|DeactivateSpotlight)
  (Development|SetHiddeninGame (Variables|Default|GetBarTimer) true false))

(event EventBeginPlay
  (bind _aswi_bar_timer (Utilities|Casting|CastToWI_BarTimer (UserInterface|GetUserWidgetObject (Variables|Default|GetBarTimer))))
  (Variables|Default|SetBarTimerHUD _aswi_bar_timer))

(event EventTick
  (params (DeltaSeconds :type Float%20%28single-precision%29))
  (if (Variables|Default|GetIsActive)
    (bind _output_get (Variables|Default|SetTimer (- (Variables|Default|GetTimer) DeltaSeconds)))
    (Variables|/Game/_Assets/Bar/Widget/WI_BarTimer.WI_BarTimer_C|SetCurrentTime (Variables|Default|GetBarTimerHUD) _output_get)
    (if (<= (Variables|Default|GetTimer) 0.0)
      (CallFunction|Deactivate))))

(fn ConstructionScript)

(fn ActivateSpotlight
  (Development|SetHiddeninGame (Variables|Default|GetLightIndicator) false false)
  (Development|SetHiddeninGame (Variables|Default|GetTriggerSphere) false false)
  (Development|SetHiddeninGame (Variables|Default|GetCylinder) false false))

(fn DeactivateSpotlight
  (Development|SetHiddeninGame (Variables|Default|GetLightIndicator) true false)
  (Development|SetHiddeninGame (Variables|Default|GetTriggerSphere) true false)
  (Development|SetHiddeninGame (Variables|Default|GetCylinder) true false))