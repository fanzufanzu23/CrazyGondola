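; Rik NPC Blueprint that switches the character's animation state when the third-person player character enters or leaves its Box trigger.
; Overlap begin calls IdleMode, which sets IsIdleRik to false on ABP_AnimationRik, and overlap end calls ClapHand, which sets it to true.
; Both events reach the flag by casting the skeletal mesh's anim instance, leaving the animation itself to that Animation Blueprint.
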(event OnComponentBeginOverlap(Box)
  (params (OverlappedComponent :type Primitive%20Component%20Object%20Reference) (OtherActor :type Actor%20Object%20Reference) (OtherComp :type Primitive%20Component%20Object%20Reference) (OtherBodyIndex :type Integer) (bFromSweep :type Boolean) (SweepResult :type Hit%20Result%20Structure%20%28by%20ref%29))
  (if (Utilities|ClassIsChildOf (Utilities|GetClass OtherActor) "/Game/ThirdPerson/Blueprints/BP_ThirdPersonCharacter.BP_ThirdPersonCharacter_C")
    (CallFunction|IdleMode)))

(event OnComponentEndOverlap(Box)
  (params (OverlappedComponent :type Primitive%20Component%20Object%20Reference) (OtherActor :type Actor%20Object%20Reference) (OtherComp :type Primitive%20Component%20Object%20Reference) (OtherBodyIndex :type Integer))
  (if (Utilities|ClassIsChildOf (Utilities|GetClass OtherActor) "/Game/ThirdPerson/Blueprints/BP_ThirdPersonCharacter.BP_ThirdPersonCharacter_C")
    (CallFunction|ClapHand)))

(event Custom|ClapHand
  (bind _asabp_animation_rik (Utilities|Casting|CastToABP_AnimationRik (Components|SkeletalMesh|GetAnimInstance (Variables|Default|GetSkeletalMesh))))
  (Variables|/Game/npc/rik/ABP_AnimationRik.ABP_AnimationRik_C|SetIsIdle_rik _asabp_animation_rik true))

(event Custom|IdleMode
  (bind _asabp_animation_rik (Utilities|Casting|CastToABP_AnimationRik (Components|SkeletalMesh|GetAnimInstance (Variables|Default|GetSkeletalMesh))))
  (Variables|/Game/npc/rik/ABP_AnimationRik.ABP_AnimationRik_C|SetIsIdle_rik _asabp_animation_rik false))

(event EventBeginPlay)

(event Collision|EventActorBeginOverlap
  (params (OtherActor :type Actor%20Object%20Reference)))

(event EventTick
  (params (DeltaSeconds :type Float%20%28single-precision%29)))

(fn ConstructionScript)