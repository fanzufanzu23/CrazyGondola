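; BP_TipaRandomTest is an NPC actor that switches its animation state when the third-person player character enters or leaves its Box trigger.
; Box overlap events class-check the other actor, then call InIdleTipa on entry or ExcitedTipa on exit.
; These events cast the skeletal mesh's anim instance to ABP_tipa1 and set IsIdleNPC false on entry, true on exit, opposite to what their names suggest.
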(event OnComponentBeginOverlap(Box)
  (params (OverlappedComponent :type Primitive%20Component%20Object%20Reference) (OtherActor :type Actor%20Object%20Reference) (OtherComp :type Primitive%20Component%20Object%20Reference) (OtherBodyIndex :type Integer) (bFromSweep :type Boolean) (SweepResult :type Hit%20Result%20Structure%20%28by%20ref%29))
  (if (Utilities|ClassIsChildOf (Utilities|GetClass OtherActor) "/Game/ThirdPerson/Blueprints/BP_ThirdPersonCharacter.BP_ThirdPersonCharacter_C")
    (CallFunction|InIdleTipa)))

(event OnComponentEndOverlap(Box)
  (params (OverlappedComponent :type Primitive%20Component%20Object%20Reference) (OtherActor :type Actor%20Object%20Reference) (OtherComp :type Primitive%20Component%20Object%20Reference) (OtherBodyIndex :type Integer))
  (if (Utilities|ClassIsChildOf (Utilities|GetClass OtherActor) "/Game/ThirdPerson/Blueprints/BP_ThirdPersonCharacter.BP_ThirdPersonCharacter_C")
    (CallFunction|ExcitedTipa)))

(event Custom|InIdleTipa
  (bind _asabp_tipa_1 (Utilities|Casting|CastToABP_tipa1 (Components|SkeletalMesh|GetAnimInstance (Variables|Default|GetSkeletalMesh))))
  (Variables|/Game/npc/tipa1/ABP_tipa1.ABP_tipa1_C|SetIsIdle_NPC _asabp_tipa_1 false))

(event Custom|ExcitedTipa
  (bind _asabp_tipa_1 (Utilities|Casting|CastToABP_tipa1 (Components|SkeletalMesh|GetAnimInstance (Variables|Default|GetSkeletalMesh))))
  (Variables|/Game/npc/tipa1/ABP_tipa1.ABP_tipa1_C|SetIsIdle_NPC _asabp_tipa_1 true))

(event EventBeginPlay)

(event Collision|EventActorBeginOverlap
  (params (OtherActor :type Actor%20Object%20Reference)))

(event EventTick
  (params (DeltaSeconds :type Float%20%28single-precision%29)))

(fn ConstructionScript)