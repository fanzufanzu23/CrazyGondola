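; BP_Fulippo is the bartender NPC Fulippo, who reacts when the player character comes near.
; A Box overlap filters for BP_ThirdPersonCharacter, firing HandUp on entry and returning to idle on exit.
; Both events cast the skeletal mesh's anim instance to AnimationBarManFulippo and set its IsIdle flag, leaving the animation change to that Animation Blueprint.
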(event OnComponentBeginOverlap(Box)
  (params (OverlappedComponent :type Primitive%20Component%20Object%20Reference) (OtherActor :type Actor%20Object%20Reference) (OtherComp :type Primitive%20Component%20Object%20Reference) (OtherBodyIndex :type Integer) (bFromSweep :type Boolean) (SweepResult :type Hit%20Result%20Structure%20%28by%20ref%29))
  (if (Utilities|ClassIsChildOf (Utilities|GetClass OtherActor) "/Game/ThirdPerson/Blueprints/BP_ThirdPersonCharacter.BP_ThirdPersonCharacter_C")
    (CallFunction|HandUp)))

(event OnComponentEndOverlap(Box)
  (params (OverlappedComponent :type Primitive%20Component%20Object%20Reference) (OtherActor :type Actor%20Object%20Reference) (OtherComp :type Primitive%20Component%20Object%20Reference) (OtherBodyIndex :type Integer))
  (if (Utilities|ClassIsChildOf (Utilities|GetClass OtherActor) "/Game/ThirdPerson/Blueprints/BP_ThirdPersonCharacter.BP_ThirdPersonCharacter_C")
    (CallFunction|IdleBarman1)))

(event Custom|Idle_Barman1
  (bind _asanimation_bar_man_fulippo (Utilities|Casting|CastToAnimationBarManFulippo (Components|SkeletalMesh|GetAnimInstance (Variables|Default|GetSkeletalMesh))))
  (Variables|/Game/npc/Barman1/Fulippo/AnimationBarManFulippo.AnimationBarManFulippo_C|SetIsIdle _asanimation_bar_man_fulippo true))

(event Custom|HandUp
  (bind _asanimation_bar_man_fulippo (Utilities|Casting|CastToAnimationBarManFulippo (Components|SkeletalMesh|GetAnimInstance (Variables|Default|GetSkeletalMesh))))
  (Variables|/Game/npc/Barman1/Fulippo/AnimationBarManFulippo.AnimationBarManFulippo_C|SetIsIdle _asanimation_bar_man_fulippo false))

(event EventBeginPlay)

(event Collision|EventActorBeginOverlap
  (params (OtherActor :type Actor%20Object%20Reference)))

(event EventTick
  (params (DeltaSeconds :type Float%20%28single-precision%29)))

(fn ConstructionScript)